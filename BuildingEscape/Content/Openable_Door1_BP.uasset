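; Openable door actor that swings open and closed in response to the OnOpen and OnClose events of OpenDoor.
; BeginPlay caches the starting rotation, and the DoorSwing timeline adds a yaw offset to it, so the swing is relative to the door's placement.
; Opening plays the timeline and closing reverses it.
; An Open Sound event track on the timeline plays the lock sound at the door's location.
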(event `self.ReceiveBeginPlay`
  (set `self.Initial Rotation` (`self.K2_GetActorRotation`)))

(event `self.OpenDoor.OnOpen`
  (bind (_direction _door_swing) (`Timeline|Door Swing` :!label _label)
    (:`Update`
      (`self.K2_SetActorRotation` (`KismetMathLibrary.ComposeRotators` (`self.Initial Rotation`) (`KismetMathLibrary.MakeRotator` 0.0 0.0 _door_swing))))
    (:`OpenSound`
      (`GameplayStatics.PlaySoundAtLocation` "/Game/Audio/door-lock.door-lock" (`self.K2_GetActorLocation`)))))

(event `self.OpenDoor.OnClose`
  (goto _label :!via `Reverse`))

(fn `UserConstructionScript`)